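; BP_Background provides a Background function that shifts a target widget with the mouse, creating a parallax-style effect for UI backgrounds.
; When enabled, it divides the viewport mouse position by per-axis X and Y factors, optionally negated by Invert, and sets the result as the widget's render translation.
; The Smush flag eases that translation with FInterpTo using world delta time and Speed; otherwise it snaps directly.
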(fn `Background`
  (params (Enable :type Boolean :default true) (Target :type "Widget Object Reference") (X :type "Float (double-precision)" :default 50.0) (Y :type "Float (double-precision)" :default 50.0) (Speed :type "Float (double-precision)" :default 5.0) (Smush :type Boolean :default true) (Invert :type Boolean :default true))
  (locals (`Local Enable` :type Boolean) (`Local Target` :type "Widget Object Reference") (`Local X` :type "Float (double-precision)") (`Lacal Y` :type "Float (double-precision)") (`Local Speed` :type "Float (double-precision)") (`Local Smush` :type Boolean) (`Local Invert` :type Boolean))
  (bind _rendertransform (`Widget.RenderTransform` (`local.Local Target`)))
  (bind _rendertransform_2 (`Widget.RenderTransform` (`local.Local Target`)))
  (set `local.Local Enable` Enable)
  (set `local.Local Target` Target)
  (set `local.Local X` X)
  (set `local.Lacal Y` Y)
  (set `local.Local Speed` Speed)
  (set `local.Local Smush` Smush)
  (set `local.Local Invert` Invert)
  (if (`local.Local Enable`)
    (if (`local.Local Invert`)
      (bind _returnvalue (`WidgetLayoutLibrary.GetMousePositionOnViewport` null))
      (if (`local.Local Smush`)
        (bind _returnvalue_2 (/ (`KismetMathLibrary.BreakVector2D` _returnvalue) (* (`local.Local X`) -1.0)))
        (bind _returnvalue_3 (/ (`.Y` (`KismetMathLibrary.BreakVector2D` _returnvalue)) (* (`local.Lacal Y`) -1.0)))
        (`Widget.SetRenderTranslation` (`local.Local Target`) (`KismetMathLibrary.MakeVector2D` (`KismetMathLibrary.FInterpTo` (`KismetMathLibrary.BreakVector2D` (break `WidgetTransform` _rendertransform)) _returnvalue_2 (`GameplayStatics.GetWorldDeltaSeconds` null) (`local.Local Speed`)) (`KismetMathLibrary.FInterpTo` (`.Y` (`KismetMathLibrary.BreakVector2D` (break `WidgetTransform` _rendertransform))) _returnvalue_3 (`GameplayStatics.GetWorldDeltaSeconds` null) (`local.Local Speed`))))
        (else
          (`Widget.SetRenderTranslation` (`local.Local Target`) (`KismetMathLibrary.MakeVector2D` _returnvalue_2 _returnvalue_3))))
      (else
        (bind _returnvalue_4 (`WidgetLayoutLibrary.GetMousePositionOnViewport` null))
        (if (`local.Local Smush`)
          (bind _returnvalue_5 (/ (`KismetMathLibrary.BreakVector2D` _returnvalue_4) (`local.Local X`)))
          (bind _returnvalue_6 (/ (`.Y` (`KismetMathLibrary.BreakVector2D` _returnvalue_4)) (`local.Lacal Y`)))
          (`Widget.SetRenderTranslation` (`local.Local Target`) (`KismetMathLibrary.MakeVector2D` (`KismetMathLibrary.FInterpTo` (`KismetMathLibrary.BreakVector2D` (break `WidgetTransform` _rendertransform_2)) _returnvalue_5 (`GameplayStatics.GetWorldDeltaSeconds` null) (`local.Local Speed`)) (`KismetMathLibrary.FInterpTo` (`.Y` (`KismetMathLibrary.BreakVector2D` (break `WidgetTransform` _rendertransform_2))) _returnvalue_6 (`GameplayStatics.GetWorldDeltaSeconds` null) (`local.Local Speed`))))
          (else
            (`Widget.SetRenderTranslation` (`local.Local Target`) (`KismetMathLibrary.MakeVector2D` _returnvalue_5 _returnvalue_6))))))))